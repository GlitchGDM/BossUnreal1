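; Player character for a boss fight, with camera-relative movement, mouse look, jumping, cooldown-limited fireball shooting, and a P key that starts boss mode.
; Boss bullet hits cost a life and briefly lock movement, jumping and shooting, ignoring further hits meanwhile.
; Losing all lives or touching the boss disables the player, notifies GameModeBoss and reloads BossLevel after a delay.
; Hit and death reactions are driven by flags set on PlayerAnimBP.
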(event Collision|EventHit
  (params (MyComp :type Primitive%20Component%20Object%20Reference) (Other :type Actor%20Object%20Reference) (OtherComp :type Primitive%20Component%20Object%20Reference) (bSelfMoved :type Boolean) (HitLocation :type Vector :default "0, 0, 0") (HitNormal :type Vector :default "0, 0, 0") (NormalImpulse :type Vector :default "0, 0, 0") (Hit :type Hit%20Result%20Structure%20%28by%20ref%29))
  ;[1 0.7026 0.3783] Check Hit or Kill
  (if (Variables|Default|GetcanMove)
    (if (Actor|ActorHasTag Other "BulletBoss")
      (Actor|DestroyActor Other)
      (Variables|Default|SetbossBullet Other)
      (Variables|Default|Setlifes (- (Variables|Default|Getlifes) 1))
      (if (> (Variables|Default|Getlifes) 0)
        (bind _asplayer_anim_bp (Utilities|Casting|CastToPlayerAnimBP (Components|SkeletalMesh|GetAnimInstance (Variables|Character|GetMesh))))
        (if (not (Variables|/Game/Blueprints/PlayerAnimBP.PlayerAnimBP_C|Getdie _asplayer_anim_bp))
          (Variables|/Game/Blueprints/PlayerAnimBP.PlayerAnimBP_C|SetenemyBullet _asplayer_anim_bp (Variables|Default|GetbossBullet))
          (Variables|/Game/Blueprints/PlayerAnimBP.PlayerAnimBP_C|SetisHit _asplayer_anim_bp true)
          (Variables|Default|SetcanMove false)
          (Variables|Default|SetcanShoot false)
          (Variables|Default|SetcanJump_1 false)
          (Utilities|FlowControl|Delay 0.05)
          (Utilities|FlowControl|Delay 0.9)
          (Variables|Default|SetcanMove true)
          (Variables|Default|SetcanShoot true)
          (Variables|Default|SetcanJump_1 true))
        (else
          (bind _asplayer_anim_bp_2 (Utilities|Casting|CastToPlayerAnimBP (Components|SkeletalMesh|GetAnimInstance (Variables|Character|GetMesh)) :!label _label))
          (if (not (Variables|/Game/Blueprints/PlayerAnimBP.PlayerAnimBP_C|Getdie _asplayer_anim_bp_2))
            (Variables|/Game/Blueprints/PlayerAnimBP.PlayerAnimBP_C|SetenemyBullet _asplayer_anim_bp_2 (Variables|Default|GetbossBullet))
            (Variables|/Game/Blueprints/PlayerAnimBP.PlayerAnimBP_C|Setdie _asplayer_anim_bp_2 true)
            (Variables|Default|SetcanMove false)
            (Variables|Default|SetcanRotate false)
            (Variables|Default|SetcanShoot false)
            (Variables|Default|SetcanJump_1 false)
            (Collision|SetActorEnableCollision false)
            (bind _asgame_mode_boss (Utilities|Casting|CastToGameModeBoss (Game|GetGameMode)))
            (Variables|/Game/Blueprints/GameModeBoss.GameModeBoss_C|SetisPlayerAlive _asgame_mode_boss false)
            (Utilities|FlowControl|Delay 3.0)
            (Game|OpenLevel(byName) "BossLevel"))))
      (elif (Actor|ActorHasTag Other "Boss")
        (Variables|Default|Setlifes 0)
        (goto _label)))))

(event Input|ActionEvents|InputActionJumpAction
  (params (Key :type Key%20Structure))
  ;[0.2889 0.9402 1] Player Jump
  (:Pressed
    (if (Variables|Default|GetcanJump_1)
      (Character|Jump))))

(event Input|ActionEvents|InputActionFireAction
  (params (Key :type Key%20Structure))
  ;[1 0.224 0.224] Shoot Fireball
  (:Pressed
    (if (Variables|Default|GetcanShoot)
      (Variables|Default|SetcanShoot false)
      (Game|SpawnActorfromClass "/Game/Blueprints/Bp_BullerPlayer.Bp_BullerPlayer_C" (Transformation|GetWorldTransform (Variables|Default|GetShootingSpawn)) "Undefined" 0 0)
      (Utilities|FlowControl|Delay 0.5)
      (Variables|Default|SetcanShoot true))))

(event Input|AxisEvents|InputAxisUpMove
  (params (AxisValue :type Float%20%28single-precision%29))
  ;[0.4078 1 0.4995] Player Movement
  (if (Variables|Default|GetcanMove)
    (Pawn|Input|AddMovementInput (Math|Vector|GetForwardVector (Math|Rotator|MakeRotator 0.0 0.0 (.Yaw (Math|Rotator|BreakRotator (Pawn|GetControlRotation :!class /Script/Engine.Pawn))))) AxisValue false)))

(event Input|AxisEvents|InputAxisRightMove
  (params (AxisValue :type Float%20%28single-precision%29))
  ;[0.4078 1 0.4995] Player Movement
  (if (Variables|Default|GetcanMove)
    (Pawn|Input|AddMovementInput (Math|Vector|GetRightVector (Math|Rotator|MakeRotator 0.0 0.0 (.Yaw (Math|Rotator|BreakRotator (Pawn|GetControlRotation :!class /Script/Engine.Pawn))))) AxisValue false)))

(event Input|AxisEvents|InputAxisLookRightMouse
  (params (AxisValue :type Float%20%28single-precision%29))
  ;[0.782 0.3441 1] Player Camera Rotation
  (if (Variables|Default|GetcanRotate)
    (Pawn|Input|AddControllerYawInput AxisValue)))

(event Input|AxisEvents|InputAxisLookUpMouse
  (params (AxisValue :type Float%20%28single-precision%29))
  ;[0.782 0.3441 1] Player Camera Rotation
  (if (Variables|Default|GetcanRotate)
    (Pawn|Input|AddControllerPitchInput AxisValue)))

(event Input|KeyboardEvents|P
  (params (Key :type Key%20Structure))
  ;[0.717 1 0.154] Start Boss
  (:Released
    (bind _asgame_mode_boss (Utilities|Casting|CastToGameModeBoss (Game|GetGameMode)))
    (Variables|/Game/Blueprints/GameModeBoss.GameModeBoss_C|SetstartBossMode _asgame_mode_boss true)))

(fn ConstructionScript)