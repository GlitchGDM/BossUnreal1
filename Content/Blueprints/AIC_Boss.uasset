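; AI controller for the boss that runs BT_BossBehaviour on possess and drives its currentStage blackboard key, starting at stage 0.
; Tick polls GameModeBoss, setting stage 2 or 3 at health thresholds.
; While StartBossMode is set, a three-second Delay writes stage 1, even at low health.
; The zero-health StopLogic call sits inside the stage 2 range check, so it is unreachable.
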(event EventTick
  (params (DeltaSeconds :type Float%20%28single-precision%29))
  (bind _asgame_mode_boss (Utilities|Casting|CastToGameModeBoss (Game|GetGameMode)))
  (if (<= (Variables|/Game/Blueprints/GameModeBoss.GameModeBoss_C|GetBossHealth _asgame_mode_boss) 0.2)
    (Class|BlackboardComponent|SetValueasInt (AI|GetBlackboard self) (Utilities|Name|MakeLiteralName "currentStage") 3))
  (if (and (<= (Variables|/Game/Blueprints/GameModeBoss.GameModeBoss_C|GetBossHealth _asgame_mode_boss) 0.5) (> (Variables|/Game/Blueprints/GameModeBoss.GameModeBoss_C|GetBossHealth _asgame_mode_boss) 0.2))
    (Class|BlackboardComponent|SetValueasInt (AI|GetBlackboard self) (Utilities|Name|MakeLiteralName "currentStage") 2)
    (if (<= (Variables|/Game/Blueprints/GameModeBoss.GameModeBoss_C|GetBossHealth _asgame_mode_boss) 0.0)
      (AI|Logic|StopLogic (Variables|Default|GetBrainComponent) "")
      (else
        (if (Variables|/Game/Blueprints/GameModeBoss.GameModeBoss_C|GetstartBossMode _asgame_mode_boss) :!label _label
          (Utilities|FlowControl|Delay 3.0)
          (Class|BlackboardComponent|SetValueasInt (AI|GetBlackboard self) (Utilities|Name|MakeLiteralName "currentStage") 1))))
    (else
      (goto _label))))

(event EventOnPossess
  (params (PossessedPawn :type Pawn%20Object%20Reference))
  (Utilities|Casting|CastToBoss PossessedPawn)
  (AI|RunBehaviorTree "/Game/BehaviourTrees/BT_BossBehaviour.BT_BossBehaviour")
  (Class|BlackboardComponent|SetValueasInt (AI|GetBlackboard self) (Utilities|Name|MakeLiteralName "currentStage")))

(fn ConstructionScript)