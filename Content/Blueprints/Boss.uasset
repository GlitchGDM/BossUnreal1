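; Boss actor that spins its four-sided shooter rig and publishes the shooter transforms to GameModeBoss every Tick.
; Collision stays off until the game mode's StartBossMode flag enables it and starts BossAnimBP.
; Hit destroys player bullets and, behind a StartBoss check that Tick clears after activation, lowers game-mode BossHealth and drives hit and death animation flags.
; Face-player logic is left unconnected.
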(event Collision|EventHit
  (params (MyComp :type Primitive%20Component%20Object%20Reference) (Other :type Actor%20Object%20Reference) (OtherComp :type Primitive%20Component%20Object%20Reference) (bSelfMoved :type Boolean) (HitLocation :type Vector :default "0, 0, 0") (HitNormal :type Vector :default "0, 0, 0") (NormalImpulse :type Vector :default "0, 0, 0") (Hit :type Hit%20Result%20Structure%20%28by%20ref%29))
  (if (Variables|Default|GetstartBoss)
    ;[1 0.6845 0.3939] On-Bullet Hit
    (bind _asboss_anim_bp (Utilities|Casting|CastToBossAnimBP (Components|SkeletalMesh|GetAnimInstance (Variables|Character|GetMesh))))
    (if (not (Variables|/Game/Blueprints/BossAnimBP.BossAnimBP_C|Getdeath _asboss_anim_bp))
      (Variables|/Game/Blueprints/BossAnimBP.BossAnimBP_C|SetisHit _asboss_anim_bp true)
      (if (Actor|ActorHasTag Other "BulletPlayer")
        (bind _asbullet_player (Utilities|Casting|CastTobulletPlayer Other))
        (Actor|DestroyActor _asbullet_player)
        (bind _asgame_mode_boss (Utilities|Casting|CastToGameModeBoss (Game|GetGameMode)))
        (Variables|/Game/Blueprints/GameModeBoss.GameModeBoss_C|SetBossHealth _asgame_mode_boss (- (Variables|/Game/Blueprints/GameModeBoss.GameModeBoss_C|GetBossHealth _asgame_mode_boss) (Variables|Default|GetBulletDamage)))
        (if (<= (Variables|/Game/Blueprints/GameModeBoss.GameModeBoss_C|GetBossHealth _asgame_mode_boss) 0.0)
          (Variables|/Game/Blueprints/BossAnimBP.BossAnimBP_C|Setdeath _asboss_anim_bp true)
          (Collision|SetActorEnableCollision false))
        (elif (not (Actor|ActorHasTag Other "Player"))
          (Actor|DestroyActor Other))))
    (elif (Actor|ActorHasTag Other "BulletPlayer")
      (bind _asbullet_player_2 (Utilities|Casting|CastTobulletPlayer Other))
      (Actor|DestroyActor _asbullet_player_2))))

(event EventBeginPlay
  (Collision|SetActorEnableCollision false))

(event EventTick
  (params (DeltaSeconds :type Float%20%28single-precision%29))
  (bind _asgame_mode_boss (Utilities|Casting|CastToGameModeBoss (Game|GetGameMode)))
  (Variables|/Game/Blueprints/GameModeBoss.GameModeBoss_C|SetshootFrontPos _asgame_mode_boss (Transformation|GetWorldTransform (Variables|Default|GetFrontShooter)))
  (Variables|/Game/Blueprints/GameModeBoss.GameModeBoss_C|SetshootBackPos _asgame_mode_boss (Transformation|GetWorldTransform (Variables|Default|GetBackShooter)))
  (Variables|/Game/Blueprints/GameModeBoss.GameModeBoss_C|SetshootLeftPos _asgame_mode_boss (Transformation|GetWorldTransform (Variables|Default|GetLeftShooter)))
  (Variables|/Game/Blueprints/GameModeBoss.GameModeBoss_C|SetshootRightPos _asgame_mode_boss (Transformation|GetWorldTransform (Variables|Default|GetRightShooter)))
  (Transformation|AddLocalRotation (Variables|Default|GetShooter) (Math|Rotator|MakeRotator 0.0 0.0 (* DeltaSeconds (Variables|Default|GetrotationSpeed))) false false)
  (if (Variables|/Game/Blueprints/GameModeBoss.GameModeBoss_C|GetstartBossMode _asgame_mode_boss)
    (bind _output_get (Variables|Default|SetstartBoss (Variables|/Game/Blueprints/GameModeBoss.GameModeBoss_C|GetstartBossMode _asgame_mode_boss)))
    (bind _asboss_anim_bp (Utilities|Casting|CastToBossAnimBP (Components|SkeletalMesh|GetAnimInstance (Variables|Character|GetMesh))))
    (bind _output_get_2 (Variables|/Game/Blueprints/BossAnimBP.BossAnimBP_C|SetstartBoss _asboss_anim_bp _output_get))
    (if _output_get_2
      (Collision|SetActorEnableCollision true)
      (Variables|Default|SetstartBoss false))))

(fn ConstructionScript)